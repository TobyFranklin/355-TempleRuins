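; Elevator actor that raises and lowers a platform inside a procedurally built shaft, driven by turn-on and turn-off events.
; The construction script stacks instanced walls per floor, leaving opposite openings at bottom and top, and derives travel height from floor count.
; A timeline plays or reverses to move the platform, rate-scaled for consistent velocity at any height.
; Collider overlap toggles first-person player input, though the interact event is empty.
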(event OnComponentBeginOverlap(Collider)
  (params (OverlappedComponent :type Primitive%20Component%20Object%20Reference) (OtherActor :type Actor%20Object%20Reference) (OtherComp :type Primitive%20Component%20Object%20Reference) (OtherBodyIndex :type Integer) (bFromSweep :type Boolean) (SweepResult :type Hit%20Result%20Structure%20%28by%20ref%29))
  (Utilities|Casting|CastToFirstPersonCharacter OtherActor)
  (Input|EnableInput (Game|GetPlayerController 0)))

(event OnComponentEndOverlap(Collider)
  (params (OverlappedComponent :type Primitive%20Component%20Object%20Reference) (OtherActor :type Actor%20Object%20Reference) (OtherComp :type Primitive%20Component%20Object%20Reference) (OtherBodyIndex :type Integer))
  (Utilities|Casting|CastToFirstPersonCharacter OtherActor)
  (Input|DisableInput (Game|GetPlayerController 0)))

(event EventPlayerWantstoInteract
  (params (Player :type First%20Person%20Character%20Object%20Reference)))

(event EventTurnon
  ;[1 1 1] Moves the elevator when turn on/turn off is called
  (bind _percent (Timeline|Elevate Play)
    (:Update
      (Transformation|SetRelativeLocation (Variables|Default|GetMover) (Math|Vector|MakeVector 0.0 0.0 (* _percent (Variables|Default|GetMax%20Height))) false false))))

(event EventTurnOff
  ;[1 1 1] Moves the elevator when turn on/turn off is called
  (bind _percent (Timeline|Elevate Reverse)
    (:Update
      (Transformation|SetRelativeLocation (Variables|Default|GetMover) (Math|Vector|MakeVector 0.0 0.0 (* _percent (Variables|Default|GetMax%20Height))) false false))))

(event EventBeginPlay
  (Components|Timeline|SetPlayRate (Variables|Default|GetElevate) (/ (Variables|Default|GetElevator%20Velocity) (Variables|Default|GetMax%20Height))))

(event Input|ActionEvents|InputActionInteract
  (params (Key :type Key%20Structure)))

(fn ConstructionScript
  (bind _wall_instanced_mesh (Variables|Default|GetWall%20Instanced%20MEsh))
  (Variables|Default|SetMax%20Height (* (Variables|Default|GetMax%20Floors) 4e+02))
  (for _index (range 0 (Variables|Default|GetMax%20Floors))
    (bind _output_get (LocalVariables|SetCurrent%20Floor _index))
    (LocalVariables|SetCurrent%20z (* _output_get 4e+02))
    ;[1 1 1] Left Wall
    (Components|InstancedStaticMesh|AddInstance _wall_instanced_mesh (Math|Transform|MakeTransform (Math|Vector|MakeVector -2e+02 2e+02 (LocalVariables|GetCurrent%20z)) "0, 0, 0" "1,1,1"))
    ;[1 1 1] Right Wall
    (Components|InstancedStaticMesh|AddInstance _wall_instanced_mesh (Math|Transform|MakeTransform (Math|Vector|MakeVector -2e+02 -2e+02 (LocalVariables|GetCurrent%20z)) "0, 0, 0" "1,1,1"))
    ;[1 1 1] Back Wall
    (if (!= (LocalVariables|GetCurrent%20Floor) (Variables|Default|GetMax%20Floors))
      (Components|InstancedStaticMesh|AddInstance _wall_instanced_mesh (Math|Transform|MakeTransform (Math|Vector|MakeVector -2e+02 2e+02 (LocalVariables|GetCurrent%20z)) "0,-90.000000, 0" "1,1,1")))
    ;[1 1 1] Front Wall
    (if (not (== (LocalVariables|GetCurrent%20Floor) 0))
      (Components|InstancedStaticMesh|AddInstance _wall_instanced_mesh (Math|Transform|MakeTransform (Math|Vector|MakeVector 2e+02 2e+02 (LocalVariables|GetCurrent%20z)) "0,-90.000000, 0" "1,1,1")))))