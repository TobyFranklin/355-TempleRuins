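; A lever Blueprint that the player flips with the Interact input to toggle another actor on or off.
; A Box overlap enables input only while the FirstPersonCharacter is inside it.
; On press, it sends TurnOn or TurnOff through the ToggleableObject interface to a referenced actor, then flips IsOn, which starts false.
; The TurningOn timeline plays or reverses to rotate the Handle.
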(event OnComponentBeginOverlap(Box)
  (params (OverlappedComponent :type Primitive%20Component%20Object%20Reference) (OtherActor :type Actor%20Object%20Reference) (OtherComp :type Primitive%20Component%20Object%20Reference) (OtherBodyIndex :type Integer) (bFromSweep :type Boolean) (SweepResult :type Hit%20Result%20Structure%20%28by%20ref%29))
  (Utilities|Casting|CastToFirstPersonCharacter OtherActor)
  (Input|EnableInput (Game|GetPlayerController 0)))

(event OnComponentEndOverlap(Box)
  (params (OverlappedComponent :type Primitive%20Component%20Object%20Reference) (OtherActor :type Actor%20Object%20Reference) (OtherComp :type Primitive%20Component%20Object%20Reference) (OtherBodyIndex :type Integer))
  (Utilities|Casting|CastToFirstPersonCharacter OtherActor)
  (Input|DisableInput (Game|GetPlayerController 0)))

(event Input|ActionEvents|InputActionInteract
  (params (Key :type Key%20Structure :default "None"))
  (bind _other_actors_controlled_by_this_actor (Variables|Default|GetOther%20Actors%20Controlled%20BY%20this%20Actor))
  (:Pressed
    ;[1 1 1] Tests to see if the other actor is valid, then calls the turn on/turn off fuction based on the state of the lever
    (Utilities|IsValid _other_actors_controlled_by_this_actor
      (:Is%20Valid
        (if (Utilities|DoesObjectImplementInterface _other_actors_controlled_by_this_actor "/Game/Blueprints/Interfaces/ToggleableObject.ToggleableObject_C")
          (if (Variables|Default|GetIsOn)
            (Class|ToggleableObject|TurnOff(Message) _other_actors_controlled_by_this_actor)
            (else
              (Class|ToggleableObject|Turnon(Message) _other_actors_controlled_by_this_actor)))
          ;[1 1 1] Swaps isOn
          (if (Variables|Default|GetIsOn)
            (Variables|Default|SetIsOn false)
            ;[1 1 1] Moves the lever
            (bind _rotation_of_socket (Timeline|Turning%20On Reverse)
              (:Update
                (Transformation|SetRelativeRotation (Variables|Default|GetHandle) (Math|Rotator|MakeRotator 0.0 _rotation_of_socket 0.0) false false)))
            (else
              (Variables|Default|SetIsOn true)
              (Timeline|Turning%20On Play))))))))

(fn ConstructionScript
  (Variables|Default|SetIsOn false))