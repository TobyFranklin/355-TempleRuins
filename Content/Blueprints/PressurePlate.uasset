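; Pressure plate actor that switches a linked actor on while something overlaps its Box and off when an overlap ends.
; It messages the referenced actor through the ToggleableObject interface, with no filter on the overlapping actor.
; A timeline drives the Plate mesh's relative Z, playing on begin and reversing on end, only when the linked actor is valid and implements the interface.
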(event OnComponentBeginOverlap(Box)
  (params (OverlappedComponent :type Primitive%20Component%20Object%20Reference) (OtherActor :type Actor%20Object%20Reference) (OtherComp :type Primitive%20Component%20Object%20Reference) (OtherBodyIndex :type Integer) (bFromSweep :type Boolean) (SweepResult :type Hit%20Result%20Structure%20%28by%20ref%29))
  (bind _other_actors_controlled_by_this_actor (Variables|Default|GetOther%20Actors%20Controlled%20BY%20this%20Actor))
  (Utilities|IsValid _other_actors_controlled_by_this_actor
    (:Is%20Valid
      (if (Utilities|DoesObjectImplementInterface _other_actors_controlled_by_this_actor "/Game/Blueprints/ToggleableObject.ToggleableObject_C")
        (Class|ToggleableObject|Turnon(Message) _other_actors_controlled_by_this_actor)
        (bind _location_of_plate (Timeline|Timeline_0 Play)
          (:Update
            (Transformation|SetRelativeLocation (Variables|Default|GetPlate) (Math|Vector|MakeVector 0.0 0.0 _location_of_plate) false false)))))))

(event OnComponentEndOverlap(Box)
  (params (OverlappedComponent :type Primitive%20Component%20Object%20Reference) (OtherActor :type Actor%20Object%20Reference) (OtherComp :type Primitive%20Component%20Object%20Reference) (OtherBodyIndex :type Integer))
  (bind _other_actors_controlled_by_this_actor (Variables|Default|GetOther%20Actors%20Controlled%20BY%20this%20Actor))
  (Utilities|IsValid _other_actors_controlled_by_this_actor
    (:Is%20Valid
      (if (Utilities|DoesObjectImplementInterface _other_actors_controlled_by_this_actor "/Game/Blueprints/ToggleableObject.ToggleableObject_C")
        (Class|ToggleableObject|TurnOff(Message) _other_actors_controlled_by_this_actor)
        (bind _location_of_plate (Timeline|Timeline_0 Reverse)
          (:Update
            (Transformation|SetRelativeLocation (Variables|Default|GetPlate) (Math|Vector|MakeVector 0.0 0.0 _location_of_plate) false false)))))))

(fn ConstructionScript)