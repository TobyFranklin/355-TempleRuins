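; Slime actor Blueprint with a simple state variable, meant to chase the FirstPersonCharacter but currently not moving.
; BeginPlay, and Tick while Idle, call PathfindToPlayer, which only looks up the player actor and checks its validity.
; The AI MoveTo that would re-path on success or failure is disconnected, so it never runs.
; ChangeState simply sets State and is not called here.
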(event Custom|Pathfind%20to%20player
  (bind _returnvalue (Actor|GetActorOfClass "/Game/Blueprints/PlayerandGame/FirstPersonCharacter.FirstPersonCharacter_C"))
  (Utilities|IsValid _returnvalue))

(event EventBeginPlay
  (CallFunction|PathfindtoPlayer))

(event EventTick
  (params (DeltaSeconds :type Float%20%28single-precision%29))
  (switch Utilities|FlowControl|Switch|SwitchonSlimeStates (Variables|Default|GetState)
    (:NewEnumerator0
      (CallFunction|PathfindtoPlayer))))

(fn ConstructionScript)

(fn ChangeState
  (params (New%20State :type SlimeStates%20Enum :default "NewEnumerator0"))
  (Variables|Default|SetState New%20State))