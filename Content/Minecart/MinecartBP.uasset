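; Rideable minecart that the player drives forward and backward along a spline track, with controller-driven look.
; Its Construction Script builds the track from spline mesh segments with clamped tangents.
; Each Tick, input accelerates velocity, an Euler step advances spline distance, and the Mover follows; both clamps are unconnected.
; Interacting possesses the cart and destroys the player; pressing Interact inside spawns and possesses a new FirstPersonCharacter at the camera.
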(event EventPlayerWantstoInteract
  (params (Player :type First%20Person%20Character%20Object%20Reference))
  ;[1 1 1] Get in minecart
  (Pawn|Possess (Pawn|GetController Player) self)
  (Actor|DestroyActor Player))

(event EventTick
  (params (DeltaSeconds :type Float%20%28single-precision%29))
  ;[1 1 1] Moves the minecart based on its speed and user input
  (CallFunction|Accelerate DeltaSeconds)
  (CallFunction|EulerStep DeltaSeconds)
  (CallFunction|PositionCart))

(event Input|ActionEvents|InputActionInteract
  (params (Key :type Key%20Structure :default "None"))
  (bind _camera (Variables|Default|GetCamera))
  (bind _returnvalue (Transformation|GetWorldTransform _camera))
  ;[1 1 1] Get out of minecart
  (:Pressed
    (bind _returnvalue_2 (Game|SpawnActorfromClass "/Game/Blueprints/FirstPersonCharacter.FirstPersonCharacter_C" (Math|Transform|MakeTransform (.location _returnvalue) (.rotation _returnvalue) "1,1,1") "Undefined" (Components|GetOwner) 0))
    (Pawn|Possess (Pawn|GetController) _returnvalue_2)))

(event Input|ActionEvents|InputActionForward
  (params (Key :type Key%20Structure :default "None"))
  (:Pressed
    (Variables|Default|SetPlayerWantsToMoveForward true))
  (:Released
    (Variables|Default|SetPlayerWantsToMoveForward false)))

(event Input|ActionEvents|InputActionBackward
  (params (Key :type Key%20Structure :default "None"))
  (:Pressed
    (Variables|Default|SetPlayerWantsToMoveBackward true))
  (:Released
    (Variables|Default|SetPlayerWantsToMoveBackward false)))

(event Input|AxisEvents|InputAxisTurn
  (params (AxisValue :type Float%20%28single-precision%29))
  ;[1 1 1] Mouse look
  (Pawn|Input|AddControllerYawInput AxisValue))

(event Input|AxisEvents|InputAxisLookUp
  (params (AxisValue :type Float%20%28single-precision%29))
  ;[1 1 1] Mouse look
  (Pawn|Input|AddControllerPitchInput AxisValue))

(event Input|AxisEvents|InputAxisTurnRate
  (params (AxisValue :type Float%20%28single-precision%29))
  ;[1 1 1] Stick Look
  (Pawn|Input|AddControllerYawInput (* AxisValue 45.0 (Utilities|Time|GetWorldDeltaSeconds))))

(event Input|AxisEvents|InputAxisLookUpRate
  (params (AxisValue :type Float%20%28single-precision%29))
  ;[1 1 1] Stick Look
  (Pawn|Input|AddControllerPitchInput (* AxisValue 45.0 (Utilities|Time|GetWorldDeltaSeconds))))

(fn ConstructionScript
  (bind _spline (Variables|Default|GetSpline))
  (bind _spline_2 (Variables|Default|GetSpline))
  (for _index (range 0 (Math|Float|Truncate (/ (Spline|GetSplineLength (Variables|Default|GetSpline)) (Variables|Default|GetLength%20of%20Piece))))
    (bind _returnvalue (AddComponent|AddSplineMeshComponent false))
    (SplineMesh|SetStartandEnd _returnvalue (Spline|GetLocationatDistanceAlongSpline _spline_2 (* _index (Variables|Default|GetLength%20of%20Piece)) "Local") (Math|Vector|ClampVectorSize (Spline|GetTangentatDistanceAlongSpline _spline_2 (* _index (Variables|Default|GetLength%20of%20Piece)) "Local") 0.0 (Variables|Default|GetLength%20of%20Piece)) (Spline|GetLocationatDistanceAlongSpline _spline (* (+ _index 1) (Variables|Default|GetLength%20of%20Piece)) "Local") (Math|Vector|ClampVectorSize (Spline|GetTangentatDistanceAlongSpline _spline (* (+ _index 1) (Variables|Default|GetLength%20of%20Piece)) "Local") 0.0 (Variables|Default|GetLength%20of%20Piece)) true :!class /Script/Engine.SplineMeshComponent)
    (CallFunction|PositionCart)))

(fn PositionCart
  (bind _position_on_spline (Variables|Default|GetPosition%20on%20Spline))
  (Transformation|SetRelativeLocationAndRotation (Variables|Default|GetMover) (Spline|GetLocationatDistanceAlongSpline (Variables|Default|GetSpline) _position_on_spline "Local") (Spline|GetRotationatDistanceAlongSpline (Variables|Default|GetSpline) _position_on_spline "Local") false false))

(fn EulerStep
  (params (dt :type Float%20%28single-precision%29))
  ;[1 1 1] Updates the carts posistion based on velocity and delta time
  (Variables|Default|SetPosition%20on%20Spline (+ (Variables|Default|GetPosition%20on%20Spline) (* dt (Variables|Default|GetVelocity)))))

(fn Accelerate
  (params (Dt :type Float%20%28single-precision%29))
  ;[1 1 1] Add acceleration in a specified direction and adds it to velocity. Also caps velocity at MaxVelocity
  (if (Variables|Default|GetPlayerWantsToMoveForward)
    (LocalVariables|SetDir 1.0))
  (if (Variables|Default|GetPlayerWantsToMoveBackward)
    (LocalVariables|SetDir (- (LocalVariables|GetDir) 1.0)))
  (Variables|Default|SetVelocity (+ (Variables|Default|GetVelocity) (* (LocalVariables|GetDir) Dt (Variables|Default|GetAcceleration)))))