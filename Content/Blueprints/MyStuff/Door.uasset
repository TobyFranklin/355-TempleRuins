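; Hinged door that the player opens and closes with Interact, or that other logic drives through Trigger, Turnon and TurnOff events.
; A box overlap enables input for the first-person character, which is cached every Tick.
; Interact compares player and hinge world Y to play one of two swing timelines, reversing by current yaw sign to close.
; The external events use a separate single-direction timeline; all timelines set SnapPoint's relative yaw.
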(event OnComponentBeginOverlap(Box)
  (params (OverlappedComponent :type Primitive%20Component%20Object%20Reference) (OtherActor :type Actor%20Object%20Reference) (OtherComp :type Primitive%20Component%20Object%20Reference) (OtherBodyIndex :type Integer) (bFromSweep :type Boolean) (SweepResult :type Hit%20Result%20Structure%20%28by%20ref%29))
  (Utilities|Casting|CastToFirstPersonCharacter OtherActor)
  (Input|EnableInput (Game|GetPlayerController 0)))

(event OnComponentEndOverlap(Box)
  (params (OverlappedComponent :type Primitive%20Component%20Object%20Reference) (OtherActor :type Actor%20Object%20Reference) (OtherComp :type Primitive%20Component%20Object%20Reference) (OtherBodyIndex :type Integer))
  (Utilities|Casting|CastToFirstPersonCharacter OtherActor)
  (Input|DisableInput (Game|GetPlayerController 0)))

(event EventTurnon
  ;[1 1 1] Opens door when called and if it is closed
  (if (not (Variables|Default|GetIsOpen))
    (Variables|Default|SetIsOpen true)
    (if (Variables|Default|GetIsOpen)
      ;[1 1 1] opens/closes the door
      (bind _open (Timeline|Timeline_1 Play)
        (:Update
          (Transformation|SetRelativeRotation (Variables|Default|GetSnap%20Point) (Math|Rotator|MakeRotator 0.0 0.0 _open) false false)))
      (else
        (Timeline|Timeline_1 Reverse)))))

(event EventTurnOff
  ;[1 1 1] Closes door when called and if it is open
  (if (Variables|Default|GetIsOpen)
    (Variables|Default|SetIsOpen false)
    (if (Variables|Default|GetIsOpen)
      ;[1 1 1] opens/closes the door
      (bind _open (Timeline|Timeline_1 Play)
        (:Update
          (Transformation|SetRelativeRotation (Variables|Default|GetSnap%20Point) (Math|Rotator|MakeRotator 0.0 0.0 _open) false false)))
      (else
        (Timeline|Timeline_1 Reverse)))))

(event EventTick
  (params (DeltaSeconds :type Float%20%28single-precision%29))
  (bind _asfirst_person_character (Utilities|Casting|CastToFirstPersonCharacter (Game|GetPlayerCharacter 0))))

(event EventTrigger
  (Variables|Default|SetIsOpen (not (Variables|Default|GetIsOpen)))
  (if (Variables|Default|GetIsOpen)
    ;[1 1 1] opens/closes the door
    (bind _open (Timeline|Timeline_1 Play)
      (:Update
        (Transformation|SetRelativeRotation (Variables|Default|GetSnap%20Point) (Math|Rotator|MakeRotator 0.0 0.0 _open) false false)))
    (else
      (Timeline|Timeline_1 Reverse))))

(event EventBeginPlay
  (Variables|Default|SetIsOpen false))

(event Input|ActionEvents|InputActionInteract
  (params (Key :type Key%20Structure))
  (:Pressed
    (if (Variables|Default|GetIsOpen)
      (Variables|Default|SetIsOpen false)
      (if (< (.yaw (Variables|/Script/Engine.SceneComponent|GetRelativeRotation (Variables|Default|GetSnap%20Point))) 0.0)
        (bind _open__otherway_ (Timeline|Open%28OtherWay%29 Reverse)
          (:Update
            (Transformation|SetRelativeRotation (Variables|Default|GetSnap%20Point) (Math|Rotator|MakeRotator 0.0 0.0 _open__otherway_) false false)))
        (else
          (bind _open (Timeline|Open Reverse)
            (:Update
              (Transformation|SetRelativeRotation (Variables|Default|GetSnap%20Point) (Math|Rotator|MakeRotator 0.0 0.0 _open) false false)))))
      (else
        (Variables|Default|SetIsOpen true)
        (if (>= (.y (Transformation|GetWorldLocation (Variables|/Script/Engine.Character|GetCapsuleComponent (stale EventTick _asfirst_person_character)))) (.y (Transformation|GetWorldLocation (Variables|Default|GetSnap%20Point))))
          (Timeline|Open%28OtherWay%29 Play)
          (else
            (Timeline|Open Play)))))))

(fn ConstructionScript)