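; LED light actor that cycles its color through red, green and blue each time its Trigger event fires.
; The construction script creates a dynamic material instance on the Cylinder and applies the current state's color.
; Trigger advances CurrentState with a Select node, then calls NewFunction0 to set the "Led Color" vector parameter.
; An unconnected switch-based version of the same cycle remains in the event graph as a comparison.
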(event EventTrigger
  ;[1 1 1] Changing the color of the material based on its last color
  (Variables|Default|SetcurrentState (Utilities|Select :Index (Variables|Default|GetcurrentState) :NewEnumerator0 "NewEnumerator1" :NewEnumerator1 "NewEnumerator2" :NewEnumerator2 "NewEnumerator0"))
  ;[1 1 1] Update the material
  (CallFunction|NewFunction0))

(fn ConstructionScript
  (bind _returnvalue (Rendering|Material|CreateDynamicMaterialInstance (Variables|Default|GetCylinder) 0 0 "None" :!class /Script/Engine.PrimitiveComponent))
  (Variables|Default|SetLED%20Material _returnvalue)
  (CallFunction|NewFunction0))

(fn NewFunction0
  (Rendering|Material|SetVectorParameterValue (Variables|Default|GetLED%20Material) "Led Color" (Utilities|Select :Index (Variables|Default|GetcurrentState) :NewEnumerator0 "(R=1.000000,G=0.009744,B=0.000000,A=1.000000)" :NewEnumerator1 "(R=0.061365,G=1.000000,B=0.000000,A=1.000000)" :NewEnumerator2 "(R=0.000000,G=0.000000,B=1.000000,A=1.000000)") :!class /Script/Engine.MaterialInstanceDynamic))