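; A drivable drone pawn that the player possesses by interacting, destroying their character, and leaves by spawning a new FirstPersonCharacter at the camera.
; Input sets movement flags; each Tick accelerates with speed-proportional drag, then moves and yaws the Mover component manually.
; Forward turning peaks at half max speed, while vertical movement is a fixed step per frame, unscaled by delta time.
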(event EventTick
  (params (DeltaSeconds :type Float%20%28single-precision%29))
  ;[1 1 1] Moves the minecart based on its speed and user input
  (CallFunction|Accelerate DeltaSeconds)
  (CallFunction|Move DeltaSeconds))

(event EventPlayerWantstoInteract
  (params (Player :type First%20Person%20Character%20Object%20Reference))
  ;[1 1 1] Get in minecart
  (Pawn|Possess (Pawn|GetController Player) self)
  (Actor|DestroyActor Player))

(event Input|ActionEvents|InputActionInteract
  (params (Key :type Key%20Structure))
  (bind _camera (Variables|Default|GetCamera))
  (bind _returnvalue (Transformation|GetWorldTransform _camera))
  ;[1 1 1] Get out of minecart
  (:Pressed
    (bind _returnvalue_2 (Game|SpawnActorfromClass "/Game/Blueprints/PlayerandGame/FirstPersonCharacter.FirstPersonCharacter_C" (Math|Transform|MakeTransform (.location _returnvalue) (.rotation _returnvalue) "1,1,1") "Undefined" (Components|GetOwner) 0))
    (Pawn|Possess (Pawn|GetController) _returnvalue_2)))

(event Input|ActionEvents|InputActionForward
  (params (Key :type Key%20Structure))
  (:Pressed
    (Variables|Default|SetMoveForward true))
  (:Released
    (Variables|Default|SetMoveForward false)))

(event Input|ActionEvents|InputActionBackward
  (params (Key :type Key%20Structure))
  (:Pressed
    (Variables|Default|SetMoveBackward true))
  (:Released
    (Variables|Default|SetMoveBackward false)))

(event Input|ActionEvents|InputActionLeft
  (params (Key :type Key%20Structure))
  (:Pressed
    (Variables|Default|SetTurnLeft true))
  (:Released
    (Variables|Default|SetTurnLeft false)))

(event Input|ActionEvents|InputActionRight
  (params (Key :type Key%20Structure))
  (:Pressed
    (Variables|Default|SetTurnRight true))
  (:Released
    (Variables|Default|SetTurnRight false)))

(event Input|ActionEvents|InputActionMoveUp
  (params (Key :type Key%20Structure))
  (:Pressed
    (Variables|Default|SetMoveUp true))
  (:Released
    (Variables|Default|SetMoveUp false)))

(event Input|ActionEvents|InputActionMoveDown
  (params (Key :type Key%20Structure))
  (:Pressed
    (Variables|Default|SetMoveDown true))
  (:Released
    (Variables|Default|SetMoveDown false)))

(event Input|AxisEvents|InputAxisTurn
  (params (AxisValue :type Float%20%28single-precision%29))
  ;[1 1 1] Mouse look
  (Pawn|Input|AddControllerYawInput AxisValue))

(event Input|AxisEvents|InputAxisLookUp
  (params (AxisValue :type Float%20%28single-precision%29))
  ;[1 1 1] Mouse look
  (Pawn|Input|AddControllerPitchInput AxisValue))

(event Input|AxisEvents|InputAxisTurnRate
  (params (AxisValue :type Float%20%28single-precision%29))
  ;[1 1 1] Stick Look
  (Pawn|Input|AddControllerYawInput (* AxisValue 45.0 (Utilities|Time|GetWorldDeltaSeconds))))

(event Input|AxisEvents|InputAxisLookUpRate
  (params (AxisValue :type Float%20%28single-precision%29))
  ;[1 1 1] Stick Look
  (Pawn|Input|AddControllerPitchInput (* AxisValue 45.0 (Utilities|Time|GetWorldDeltaSeconds))))

(fn ConstructionScript)

(fn Move
  (params (Dt :type Float%20%28single-precision%29))
  (bind _forward_velocity (Variables|Default|GetForward%20Velocity))
  (bind _maxvelocity (Variables|Default|GetMaxVelocity))
  (bind _mover (Variables|Default|GetMover))
  (bind _mover_2 (Variables|Default|GetMover))
  (bind _returnvalue (/ _maxvelocity 2.0))
  (bind _returnvalue_2 (Transformation|GetWorldLocation _mover))
  (bind _returnvalue_3 (Transformation|GetWorldRotation _mover_2))
  (bind _returnvalue_4 (* Dt _forward_velocity))
  ;[1 1 1] Updates the carts posistion based on velocity and delta time
  ;[1 1 1] Vertical MOvement
  (Variables|Default|SetVelocityUp 0.0)
  (if (Variables|Default|GetMoveUp)
    (Variables|Default|SetVelocityUp 5.0))
  (if (Variables|Default|GetMoveDown)
    (bind _output_get (Variables|Default|SetVelocityUp (- (Variables|Default|GetVelocityUp) 5.0))))
  (Transformation|SetWorldLocation (Variables|Default|GetMover) (Math|Vector|MakeVector (+ (* _returnvalue_4 (Math|Trig|Cos(Degrees) (.yaw _returnvalue_3))) (.x _returnvalue_2)) (+ (* _returnvalue_4 (Math|Trig|Sin(Degrees) (.yaw _returnvalue_3))) (.y _returnvalue_2)) (+ (.z _returnvalue_2) _output_get)) false false)
  ;[1 1 1] Sets the turn rate based on which buttons you are pressing
  (Variables|Default|SetTurnRate 0.0)
  (if (Variables|Default|GetTurnRight)
    (Variables|Default|SetTurnRate (+ (Variables|Default|GetTurnRate) 1.0)))
  (if (Variables|Default|GetTurnLeft)
    (Variables|Default|SetTurnRate (- (Variables|Default|GetTurnRate) 1.0)))
  ;[1 1 1] Rotates the vehicle
  (Transformation|SetWorldRotation (Variables|Default|GetMover) (Math|Rotator|MakeRotator 0.0 0.0 (+ (.yaw _returnvalue_3) (* (Variables|Default|GetTurnRate) (Math|Float|Absolute(Float) (* (- 1.0 (/ (Math|Float|Absolute(Float) (- _returnvalue (Variables|Default|GetForward%20Velocity))) _returnvalue)) (Variables|Default|GetTurnRate)))))) false false))

(fn Accelerate
  (params (Dt :type Float%20%28single-precision%29))
  (bind _maxvelocity (Variables|Default|GetMaxVelocity))
  ;[1 1 1] Add acceleration in a specified direction and adds it to velocity. Also caps velocity at MaxVelocity
  (Variables|Default|SetDir 0.0)
  (if (Variables|Default|GetMoveForward)
    (Variables|Default|SetDir 1.0))
  (if (Variables|Default|GetMoveBackward)
    (Variables|Default|SetDir (- (Variables|Default|GetDir) 1.0)))
  (Variables|Default|SetForward%20Velocity (Math|Float|Clamp(Float) (+ (Variables|Default|GetForward%20Velocity) (* (- (Variables|Default|GetDir) (/ (Variables|Default|GetForward%20Velocity) _maxvelocity)) (Variables|Default|GetAcceleration%20Forward) Dt)) (* -1.0 _maxvelocity) _maxvelocity)))